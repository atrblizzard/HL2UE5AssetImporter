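; Single-player game mode for Half-Life 2 style maps that handles player spawning and map start logic.
; On BeginPlay it finds entities named "logic_auto" and forwards the game mode start event to them.
; Player start selection picks a random info_player_start, preferring those flagged as master.
; Both default pawn spawn overrides raise the spawn point, spawn regardless of collision and possess the pawn immediately.
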(event `self.ReceiveBeginPlay`
  (`parent.ReceiveBeginPlay`)
  (bind _outentities (`HL2Utils.FindEntitiesByTargetName` "logic_auto"))
  (for _array_element _outentities
    (bind _aslogic_auto (cast `/HL2AssetImporter/Entities/logic_auto` _array_element))
    (`/HL2AssetImporter/Entities/logic_auto.GamemodeBeginPlay` _aslogic_auto)))

(fn `FindPlayerStart`
  (params (Player :type "Controller Object Reference") (IncomingName :type String))
  (returns (ReturnValue :type "Actor Object Reference"))
  (locals (masterSpawns :type "Array of /HL2AssetImporter/Entities/info_player_start Object Reference"))
  (bind _returnvalue (`KismetArrayLibrary.Array_Length` (`local.masterSpawns`)))
  (bind _outactors (`GameplayStatics.GetAllActorsOfClass` "/HL2AssetImporter/Entities/info_player_start.info_player_start_C"))
  (set `local.masterSpawns` (`|MakeArray`))
  (for _array_element _outactors
    (if (`/HL2AssetImporter/Entities/info_player_start.IsMaster` _array_element)
      (`KismetArrayLibrary.Array_Add` (`local.masterSpawns`) _array_element)))
  (if (> _returnvalue 0)
    (return (`|GetArrayItem` (`local.masterSpawns`) (`KismetMathLibrary.RandomIntegerInRange` 0 (- _returnvalue 1))))
    (else
      (return (`|GetArrayItem` _outactors (`KismetMathLibrary.RandomIntegerInRange` 0 (- (`KismetArrayLibrary.Array_Length` _outactors) 1)))))))

(fn `SpawnDefaultPawnAtTransform`
  (params (NewPlayer :type "Controller Object Reference") (SpawnTransform :type "Transform Structure (by ref)"))
  (returns (ReturnValue :type "Pawn Object Reference"))
  (bind _returnvalue (`|SpawnActorFromClass` (`self.DefaultPawnClass`) (`KismetMathLibrary.ComposeTransforms` SpawnTransform (`KismetMathLibrary.MakeTransform` (0.0 0.0 100.0))) "AlwaysSpawn" "OverrideRootScale" null null))
  (`Controller.Possess` NewPlayer _returnvalue)
  (return _returnvalue))

(fn `SpawnDefaultPawnFor`
  (params (NewPlayer :type "Controller Object Reference") (StartSpot :type "Actor Object Reference"))
  (returns (ReturnValue :type "Pawn Object Reference"))
  (bind _returnvalue (`|SpawnActorFromClass` (`self.DefaultPawnClass`) (`KismetMathLibrary.ComposeTransforms` (`SceneComponent.K2_GetComponentToWorld` (`Actor.RootComponent` StartSpot)) (`KismetMathLibrary.MakeTransform` (0.0 0.0 100.0))) "AlwaysSpawn" "OverrideRootScale" null null))
  (`Controller.Possess` NewPlayer _returnvalue)
  (return _returnvalue))

(fn `UserConstructionScript`)