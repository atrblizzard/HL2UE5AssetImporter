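; HL2PlayerController is a player controller that turns keyboard and mouse input into first-person-style control of the possessed pawn.
; BeginPlay registers the HL2 Enhanced Input mapping context, while look uses legacy MouseX/MouseY axes with inverted pitch.
; Both Tick and IA_Move feed one yaw-relative AddMovementInput call.
; Jump and crouch actions call Character functions, while sprint calls HL2PlayerCharacter's BeginSprint and EndSprint.
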(event `self.ReceiveBeginPlay`
  (bind _returnvalue (subsystem `EnhancedInputLocalPlayerSubsystem`))
  (`self.ResetIgnoreMoveInput`)
  (`/Engine/EditorBlueprintResources/StandardMacros.IsValid` _returnvalue
    (:`Is Valid`
      (`EnhancedInputSubsystemInterface.AddMappingContext` _returnvalue "/HL2AssetImporter/Blueprints/HL2InputMappingContext.HL2InputMappingContext" 0 (struct)))))

(event `self.ReceiveTick`
  (params (DeltaSeconds :type "Float (single-precision)"))
  (bind (_returnvalue_roll _returnvalue_pitch _returnvalue_yaw) (`KismetMathLibrary.BreakRotator` (`self.GetControlRotation`)))
  (bind _returnvalue (`KismetMathLibrary.MakeRotator` 0.0 0.0 _returnvalue_yaw))
  (`parent.ReceiveTick` DeltaSeconds)
  (bind (_x _y) (`KismetMathLibrary.BreakVector2D` (stale `EnhancedInput|/HL2AssetImporter/Blueprints/Actions/IA_Move` ActionValue)))
  (`Pawn.AddMovementInput` (`self.K2_GetPawn`) (+ (* (`KismetMathLibrary.GetForwardVector` _returnvalue) _y) (* (`KismetMathLibrary.GetRightVector` _returnvalue) _x)) 1.0 false :!label _label))

(event `EnhancedInput|/HL2AssetImporter/Blueprints/Actions/IA_Move`
  (params (ActionValue :type "Vector2D Structure") (ElapsedSeconds :type "Float (double-precision)") (TriggeredSeconds :type "Float (double-precision)") (InputAction :type "InputAction Object Reference" :default "/HL2AssetImporter/Blueprints/Actions/IA_Move.IA_Move"))
  (:`Triggered`
    (goto _label))
  (:`Completed`
    (`Pawn.ConsumeMovementInputVector` (`self.K2_GetPawn`))))

(event `InputAxisKey|MouseX`
  (params (AxisValue :type "Float (single-precision)"))
  (`self.AddYawInput` AxisValue))

(event `InputAxisKey|MouseY`
  (params (AxisValue :type "Float (single-precision)"))
  (`self.AddPitchInput` (* AxisValue -1.0)))

(event `EnhancedInput|/HL2AssetImporter/Blueprints/Actions/IA_Jump`
  (params (ActionValue :type Boolean) (ElapsedSeconds :type "Float (double-precision)") (TriggeredSeconds :type "Float (double-precision)") (InputAction :type "InputAction Object Reference" :default "/HL2AssetImporter/Blueprints/Actions/IA_Jump.IA_Jump"))
  (bind _returnvalue (`self.K2_GetPawn`))
  (:`Triggered`
    (bind _ascharacter (cast `Character` _returnvalue))
    (`Character.Jump` _ascharacter))
  (:`Completed`
    (bind _ascharacter_2 (cast `Character` _returnvalue))
    (`Character.StopJumping` _ascharacter_2)))

(event `EnhancedInput|/HL2AssetImporter/Blueprints/Actions/IA_Crouch`
  (params (ActionValue :type Boolean) (ElapsedSeconds :type "Float (double-precision)") (TriggeredSeconds :type "Float (double-precision)") (InputAction :type "InputAction Object Reference" :default "/HL2AssetImporter/Blueprints/Actions/IA_Crouch.IA_Crouch"))
  (bind _returnvalue (`self.K2_GetPawn`))
  (:`Triggered`
    (bind _ascharacter (cast `Character` _returnvalue))
    (`Character.Crouch` _ascharacter))
  (:`Completed`
    (bind _ascharacter_2 (cast `Character` _returnvalue))
    (`Character.UnCrouch` _ascharacter_2)))

(event `EnhancedInput|/HL2AssetImporter/Blueprints/Actions/IA_Sprint`
  (params (ActionValue :type Boolean) (ElapsedSeconds :type "Float (double-precision)") (TriggeredSeconds :type "Float (double-precision)") (InputAction :type "InputAction Object Reference" :default "/HL2AssetImporter/Blueprints/Actions/IA_Sprint.IA_Sprint"))
  (bind _returnvalue (`self.K2_GetPawn`))
  (:`Triggered`
    (bind _ashl2player_character (cast `/HL2AssetImporter/Blueprints/HL2PlayerCharacter` _returnvalue))
    (`/HL2AssetImporter/Blueprints/HL2PlayerCharacter.BeginSprint` _ashl2player_character))
  (:`Completed`
    (bind _ashl2player_character_2 (cast `/HL2AssetImporter/Blueprints/HL2PlayerCharacter` _returnvalue))
    (`/HL2AssetImporter/Blueprints/HL2PlayerCharacter.EndSprint` _ashl2player_character_2)))

(fn `UserConstructionScript`)